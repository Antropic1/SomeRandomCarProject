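; BP_ServiceManager is a facade that exposes the quest system through SM-prefixed events and functions.
; Its events forward calls to QuestManager to start or auto-start quests, complete objectives, and set current, completed-objective and completed-quest widgets.
; Its getter functions return the manager's active and completed quests and those same widget references.
; It holds no quest logic of its own, acting purely as a pass-through layer.
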(event EventSMCompleteAnObjective
  (params (QuestID :type Name :default "None") (ObjectiveID :type Name :default "None"))
  (Default|QMCompleteObjective (Variables|Default|GetQuestManager) QuestID ObjectiveID))

(event EventSMStartQuest
  (params (QuestID :type Name :default "None"))
  (Default|QMStartQuest (Variables|Default|GetQuestManager) QuestID))

(event EventSMSetCompletedObjectiveWidget
  (params (completedObjective :type Widget%20Object%20Reference))
  (Default|QMSetCompletedObjectiveWidget (Variables|Default|GetQuestManager) completedObjective))

(event EventSMSetCompletedQuestWidget
  (params (CompletedQuest :type Widget%20Object%20Reference))
  (Default|QMSetCompletedQuestWidget (Variables|Default|GetQuestManager) CompletedQuest))

(event EventSMSetCurrentWidget
  (params (Widget :type Widget%20Object%20Reference))
  (Default|QMSetCurrentWidget (Variables|Default|GetQuestManager) Widget))

(event EventSMAutoStartQuests
  (Default|QMAutoStartQuests (Variables|Default|GetQuestManager)))

(fn ConstructionScript)

(fn SMGetActiveQuests(New)
  (bind _activequests (Default|QMGetActiveQuests (Variables|Default|GetQuestManager)))
  (return _activequests))

(fn SMGetCompletedObjectiveWidgett
  (bind _completedobjective (Default|QMGetCompletedObjectiveWidget (Variables|Default|GetQuestManager)))
  (return _completedobjective))

(fn SMGetCompletedQuests
  (bind _completedquests (Default|QMGetCompletedQuests (Variables|Default|GetQuestManager)))
  (return _completedquests))

(fn SMGetCompletedQuestWidgett
  (bind _completedquest (Default|QMGetCompletedQuestWidget (Variables|Default|GetQuestManager)))
  (return _completedquest))

(fn SMGetCurrentWidget
  (bind _widget (Default|QMGetCurrentWidget (Variables|Default|GetQuestManager)))
  (return _widget))