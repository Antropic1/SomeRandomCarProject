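; BP_MassTestingCharacter is a player character used as a temporary test harness for the quest system.
; On BeginPlay it finds BP_ServiceManager and auto-starts quests.
; Debug keys start the first DT_QuestDefintions quest and complete its lost amulet objectives; F, G and H are unfinished second-quest stubs.
; The I key recreates WBP_HUD with the manager, switches to UI-only input with cursor, and pauses the game.
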(event EventBeginPlay
  (bind _returnvalue (Actor|GetActorOfClass "/Game/GameplaySystems/Quest/BPs/BP_ServiceManager.BP_ServiceManager_C"))
  (bind _output_get (Variables|Default|SetBP_ServiceManager _returnvalue))
  (Default|SMAutoStartQuests _output_get))

(event Input|KeyboardEvents|E
  (params (Key :type Key%20Structure :default "None"))
  ;[0.15 0.15 0.15 0.5] This is a test implementation for updating the lost amulet quest, this will be replaced by trigerable events so this is just for testing purpose.
  (:Pressed
    (bind _outrownames (DataTable|GetDataTableRowNames "/Game/GameplaySystems/Quest/DataTables/DT_QuestDefintions.DT_QuestDefintions"))
    (Default|SMStartQuest (Variables|Default|GetBP_ServiceManager) (Utilities|Array|Get(acopy) _outrownames))))

(event Input|KeyboardEvents|R
  (params (Key :type Key%20Structure :default "None"))
  ;[0.15 0.15 0.15 0.5] This is a test implementation for updating the lost amulet quest, this will be replaced by trigerable events so this is just for testing purpose.
  (:Pressed
    (bind _outrownames (DataTable|GetDataTableRowNames "/Game/GameplaySystems/Quest/DataTables/DT_QuestDefintions.DT_QuestDefintions"))
    (Default|SMCompleteAnObjective (Variables|Default|GetBP_ServiceManager) (Utilities|Array|Get(acopy) _outrownames) "TalkToOldMan")))

(event Input|KeyboardEvents|I
  (params (Key :type Key%20Structure :default "None"))
  (bind _returnvalue (Game|GetPlayerController 0))
  ;[0.15 0.15 0.15 0.5] Add HUD to screen
  (:Pressed
    (bind _hud (Variables|Default|GetHUD)
      (:then
        (Widget|RemovefromParent _hud))
      (:else
        _))
    (bind _returnvalue_2 (UserInterface|CreateWidget "/Game/GameplaySystems/Quest/Widgets/WBP_HUD.WBP_HUD_C" 0 (Variables|Default|GetBP_ServiceManager)))
    (bind _output_get (Variables|Default|SetHUD _returnvalue_2))
    (UserInterface|Viewport|AddtoViewport _output_get 0)
    (Input|SetInputModeUIOnly _returnvalue _output_get "DoNotLock" false)
    (Variables|/Script/Engine.PlayerController|SetbShowMouseCursor _returnvalue true)
    (Game|SetGamePaused true)))

(event Input|KeyboardEvents|T
  (params (Key :type Key%20Structure :default "None"))
  ;[0.15 0.15 0.15 0.5] This is a test implementation for updating the lost amulet quest, this will be replaced by trigerable events so this is just for testing purpose.
  (:Pressed
    (bind _outrownames (DataTable|GetDataTableRowNames "/Game/GameplaySystems/Quest/DataTables/DT_QuestDefintions.DT_QuestDefintions"))
    (Default|SMCompleteAnObjective (Variables|Default|GetBP_ServiceManager) (Utilities|Array|Get(acopy) _outrownames) "FindAmulet")))

(event Input|KeyboardEvents|Y
  (params (Key :type Key%20Structure :default "None"))
  ;[0.15 0.15 0.15 0.5] This is a test implementation for updating the lost amulet quest, this will be replaced by trigerable events so this is just for testing purpose.
  (:Pressed
    (bind _outrownames (DataTable|GetDataTableRowNames "/Game/GameplaySystems/Quest/DataTables/DT_QuestDefintions.DT_QuestDefintions"))
    (Default|SMCompleteAnObjective (Variables|Default|GetBP_ServiceManager) (Utilities|Array|Get(acopy) _outrownames) "ReturnToOldMan")))

(event Input|KeyboardEvents|F
  (params (Key :type Key%20Structure :default "None"))
  ;[0.15 0.15 0.15 0.5] test for the second test quest
  (:Pressed
    (bind _outrownames (DataTable|GetDataTableRowNames "/Game/GameplaySystems/Quest/DataTables/DT_QuestDefintions.DT_QuestDefintions"))))

(event Input|KeyboardEvents|G
  (params (Key :type Key%20Structure :default "None"))
  ;[0.15 0.15 0.15 0.5] test for the second test quest
  (:Pressed
    (bind _outrownames (DataTable|GetDataTableRowNames "/Game/GameplaySystems/Quest/DataTables/DT_QuestDefintions.DT_QuestDefintions"))))

(event Input|KeyboardEvents|H
  (params (Key :type Key%20Structure :default "None"))
  ;[0.15 0.15 0.15 0.5] test for the second test quest
  (:Pressed
    (bind _outrownames (DataTable|GetDataTableRowNames "/Game/GameplaySystems/Quest/DataTables/DT_QuestDefintions.DT_QuestDefintions"))))

(fn ConstructionScript)

(fn GetPlayerHUD
  (return (Variables|Default|GetHUD)))

(fn GetServiceManager
  (return (Variables|Default|GetBP_ServiceManager)))