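; Test enemy base Blueprint that damages Player-tagged actors overlapping its capsule.
; An overlap while damage is allowed sends DamageMessage with DamageAmount, disables further damage and starts a short reset timer.
; The timer's reset event clears the handle but sets IsAbleToDamage to false again, so nothing shown here re-enables damage after the first hit.
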(event OnComponentBeginOverlap(CapsuleComponent)
  (params (OverlappedComponent :type Primitive%20Component%20Object%20Reference) (OtherActor :type Actor%20Object%20Reference) (OtherComp :type Primitive%20Component%20Object%20Reference) (OtherBodyIndex :type Integer) (bFromSweep :type Boolean) (SweepResult :type Hit%20Result%20Structure%20%28by%20ref%29))
  (if (and (Actor|ActorHasTag OtherActor "Player") (Variables|Default|GetIsAbleToDamage))
    (Class|INTDamageSystem|Damage(Message) OtherActor (Variables|Default|GetDamage%20Amount))
    (Variables|Default|SetIsAbleToDamage false)
    (bind _returnvalue (Utilities|Time|SetTimerbyEvent (delegate Custom|resetCanDamage) 2.5))
    (Variables|Default|SetResetCanDamageHandle _returnvalue)))

(event Custom|resetCanDamage
  (Variables|Default|SetIsAbleToDamage false)
  (CallFunction|ClearResetHandle))

(event Custom|ClearResetHandle
  (Utilities|Time|ClearandInvalidateTimerbyHandle (Variables|Default|GetResetCanDamageHandle)))

(fn ConstructionScript)